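; BP_MyDrone is a drone Blueprint whose graph animates its spinning wings.
; Every Tick, a Sequence adds local yaw rotation to four wing components, scaled by delta time for frame-rate independence.
; Spin rate grows with the movement component's velocity magnitude via a ratio, plus a minimum that maintains rotation at rest, all scaled by a shared multiplier.
; The Construction Script is empty, and the graph contains no flight or input logic.
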(event EventTick
  (params (DeltaSeconds :type Float%20%28single-precision%29))
  (bind _returnvalue (Pawn|GetMovementComponent))
  (bind _rotationmultiplier (Variables|Default|GetRotationMultiplier))
  (bind _minimumrotation (Variables|Default|GetMinimumRotation))
  (bind _velocityrotationratio (Variables|Default|GetVelocityRotationRatio))
  (bind _velocity (Variables|/Script/Engine.MovementComponent|GetVelocity _returnvalue))
  (bind _returnvalue_2 (Math|Vector|VectorLength _velocity))
  (bind _returnvalue_3 (* _returnvalue_2 _velocityrotationratio))
  (bind _returnvalue_4 (+ _returnvalue_3 _minimumrotation))
  (bind _returnvalue_5 (* _rotationmultiplier _returnvalue_4))
  (bind _returnvalue_6 (* _returnvalue_5 DeltaSeconds))
  ;[0.15 0.15 0.15 0.5] Drone wing anim
  (Utilities|FlowControl|Sequence
    (:then_0
      (Transformation|AddLocalRotation (Variables|Default|GetDroneWing) (Math|Rotator|MakeRotator 0.0 0.0 _returnvalue_6) false false))
    (:then_1
      (Transformation|AddLocalRotation (Variables|Default|GetDroneWing1) (Math|Rotator|MakeRotator 0.0 0.0 _returnvalue_6) false false))
    (:then_2
      (Transformation|AddLocalRotation (Variables|Default|GetDroneWing3) (Math|Rotator|MakeRotator 0.0 0.0 _returnvalue_6) false false))
    (:then_3
      (Transformation|AddLocalRotation (Variables|Default|GetDroneWing4) (Math|Rotator|MakeRotator 0.0 0.0 _returnvalue_6) false false))))

(fn ConstructionScript)